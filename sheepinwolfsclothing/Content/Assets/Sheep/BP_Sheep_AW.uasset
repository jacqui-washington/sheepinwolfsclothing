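; BP_Sheep_AW is a sheep actor that plays ambient idle sounds and can trigger a death animation.
; A random sound from an array plays at the skeletal mesh on BeginPlay, then repeats on a randomized delay loop.
; The SheepDeath event (with a debug print) and the E key both call SheepDeathAnim on the ABP_Sheep_AW anim instance.
; The construction script applies a material variation, while the movement timeline logic is disconnected.
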(event `self.ReceiveBeginPlay`
  (bind _sheepidlesound (`self.SheepIdleSound`))
  (bind _returnvalue (`SceneComponent.K2_GetComponentLocation` (`self.SK_Sheep_AW`)))
  (bind _output (`|GetArrayItem` _sheepidlesound (`KismetMathLibrary.RandomIntegerInRange` 0 (`KismetArrayLibrary.Array_Length` _sheepidlesound))))
  (`GameplayStatics.PlaySoundAtLocation` _output _returnvalue (struct) 1.0 1.0 0.0 null null null)
  (`KismetSystemLibrary.RetriggerableDelay` (`KismetMathLibrary.RandomFloatInRange` 10.0 20.0) :!label _label)
  (`GameplayStatics.PlaySoundAtLocation` _output _returnvalue (struct) 1.0 1.0 0.0 null null null)
  (goto _label))

(event `Key|E`
  (params (Key :type "Key Structure"))
  (:`Pressed`
    (bind _asabp_sheep_aw (cast `/Game/Assets/Sheep/ABP_Sheep_AW` (`SkeletalMeshComponent.GetAnimInstance` (`self.SK_Sheep_AW`)) :!label _label_2))
    (`/Game/Assets/Sheep/ABP_Sheep_AW.SheepDeathAnim` _asabp_sheep_aw)))

(event `SheepDeath`
  (`KismetSystemLibrary.PrintString` "Hello")
  (goto _label_2))

(fn `UserConstructionScript`
  (`PrimitiveComponent.SetMaterial` (`self.SK_Sheep_AW`) 0 (`self.MaterialVariation`)))